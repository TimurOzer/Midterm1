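; Swinging axes trap actor that reacts when the third-person character overlaps its Box trigger.
; On overlap, the Speed timeline rolls two static meshes in opposite directions.
; When that finishes, a capsule trace at the actor's location calls Hit on the character if it finds one.
; Leaving the Box plays a separate timeline in reverse from the end, driving the same mirrored roll.
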(event `self.Box.OnComponentBeginOverlap`
  (params (OverlappedComponent :type "PrimitiveComponent Object Reference") (OtherActor :type "Actor Object Reference") (OtherComp :type "PrimitiveComponent Object Reference") (OtherBodyIndex :type Integer) (bFromSweep :type Boolean) (SweepResult :type "HitResult Structure (by ref)"))
  (bind _returnvalue (`self.K2_GetActorLocation`))
  (cast `/Game/TimurOzer2200969/BP_ThirdPersonCharacter` OtherActor)
  (bind (_direction _newtrack_0) (`Timeline|Speed` :!via `PlayFromStart`)
    (:`Update`
      (`SceneComponent.K2_SetRelativeRotation` (`self.StaticMesh1`) (`KismetMathLibrary.MakeRotator` _newtrack_0) false false)
      (`SceneComponent.K2_SetRelativeRotation` (`self.StaticMesh`) (`KismetMathLibrary.MakeRotator` (* _newtrack_0 -1.0)) false false))
    (:`Finished`
      (bind _outhit (`KismetSystemLibrary.CapsuleTraceSingle` _returnvalue _returnvalue 200.0 200.0 "TraceTypeQuery1"))
      (bind _asbp_third_person_character (cast `/Game/TimurOzer2200969/BP_ThirdPersonCharacter` (`.HitActor` (`GameplayStatics.BreakHitResult` _outhit))))
      (`/Game/TimurOzer2200969/BP_ThirdPersonCharacter.Hit` _asbp_third_person_character))))

(event `self.Box.OnComponentEndOverlap`
  (params (OverlappedComponent :type "PrimitiveComponent Object Reference") (OtherActor :type "Actor Object Reference") (OtherComp :type "PrimitiveComponent Object Reference") (OtherBodyIndex :type Integer))
  (cast `/Game/TimurOzer2200969/BP_ThirdPersonCharacter` OtherActor)
  (bind (_direction _newtrack_0) (`Timeline|Timeline_0` :!via `ReverseFromEnd`)
    (:`Update`
      (`SceneComponent.K2_SetRelativeRotation` (`self.StaticMesh1`) (`KismetMathLibrary.MakeRotator` _newtrack_0) false false)
      (`SceneComponent.K2_SetRelativeRotation` (`self.StaticMesh`) (`KismetMathLibrary.MakeRotator` (* _newtrack_0 -1.0)) false false))))

(fn `UserConstructionScript`)