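; Maze ("Labirent") cell actor that also runs the level's time limit.
; The construction script adds flag-selected wall meshes sized from GridSize, with the ceiling nested under the south-wall branch and an optional point light under the ceiling.
; At BeginPlay, non-Generator instances play a timeline driving the LightTime parameter collection's Time value.
; When it finishes, they show a losing WinLose widget and immediately open level NewLevelOPHW.
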(event `self.ReceiveBeginPlay`
  (if (not (`self.Generator`))
    (bind (_direction _newtrack_0) (`Timeline|Timeline`)
      (:`Update`
        (`KismetMaterialLibrary.SetScalarParameterValue` "/Game/TimurOzer2200969/LightTime.LightTime" "Time" _newtrack_0))
      (:`Finished`
        (bind _returnvalue (`|CreateWidget` "/Game/TimurOzer2200969/WinLose.WinLose_C"))
        (`UserWidget.AddToViewport` _returnvalue 0)
        (set `/Game/TimurOzer2200969/WinLose.Win` false _returnvalue)
        (`GameplayStatics.OpenLevel` "NewLevelOPHW")))))

(fn `UserConstructionScript`
  (locals (WallThickness :type "Float (double-precision)") (WallLenght :type "Float (double-precision)") (WallHeight :type "Float (double-precision)" :default 500.0))
  (bind _gridsize (`self.GridSize`))
  (bind _returnvalue (/ (`local.WallLenght`) 2.0))
  (set `local.WallLenght` _gridsize)
  (set `local.WallThickness` (* _gridsize 0.1))
  (`SceneComponent.SetRelativeScale3D` (`self.StaticMesh`) (0.0 0.0 0.0))
  (if (`self.Left(West)`)
    (`AddComponent|NODE_AddStaticMeshComponent-5`))
  (if (`self.Right(East)`)
    (`AddComponent|NODE_AddStaticMeshComponent-6` :`RelativeTransform` (`KismetMathLibrary.MakeTransform` (`KismetMathLibrary.MakeVector` 0.0 (- (`local.WallLenght`) (`local.WallThickness`))))))
  (if (`self.Up(North)`)
    (`AddComponent|NODE_AddStaticMeshComponent-7` :`RelativeTransform` (`KismetMathLibrary.MakeTransform` (`KismetMathLibrary.MakeVector` 0.0 (- (`local.WallLenght`) (`local.WallThickness`))))))
  (if (`self.Down(South)`)
    (`AddComponent|NODE_AddStaticMeshComponent-8` :`RelativeTransform` (`KismetMathLibrary.MakeTransform` (`KismetMathLibrary.MakeVector` 0.0 (- (`local.WallLenght`) (`local.WallThickness`)))))
    (if (`self.Ceiling`)
      (`AddComponent|NODE_AddStaticMeshComponent-9` :`RelativeTransform` (`KismetMathLibrary.MakeTransform` (`KismetMathLibrary.MakeVector` 0.0 0.0 (- (`local.WallLenght`) (`local.WallThickness`)))))
      (if (> (`self.LightIntensity`) 0.0)
        (bind _returnvalue_2 (`AddComponent|NODE_AddPointLightComponent-1` :`RelativeTransform` (`KismetMathLibrary.MakeTransform` (`KismetMathLibrary.MakeVector` _returnvalue _returnvalue (* (`local.WallHeight`) 0.75)))))
        (`LightComponent.SetIntensity` _returnvalue_2 (`self.LightIntensity`))))))