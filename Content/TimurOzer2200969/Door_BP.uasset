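; Door Blueprint that slides open when interacted with, provided the key value stored in the third-person game mode matches the door's KeyNumber.
; BeginPlay caches the game mode; on a match, Interact plays a Timeline that lerps the mesh's relative location from StartLocation to EndLocation.
; A mismatch prints a wrong-key message, and the construction script applies the configurable Material to the mesh.
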(event `self.ReceiveBeginPlay`
  (bind _asbp_third_person_game_mode (cast `/Game/ThirdPerson/Blueprints/BP_ThirdPersonGameMode` (`GameplayStatics.GetGameMode`)))
  (set `self.As BP Third Person Game Mode` _asbp_third_person_game_mode))

(event `/Game/TimurOzer2200969/Interact.Interact`
  (if (== (`/Game/ThirdPerson/Blueprints/BP_ThirdPersonGameMode.Keys` (`self.As BP Third Person Game Mode`)) (`self.KeyNumber`))
    (bind (_direction _newtrack_0) (`Timeline|Timeline` :!via `PlayFromStart`)
      (:`Update`
        (`SceneComponent.K2_SetRelativeLocation` (`self.StaticMesh`) (`KismetMathLibrary.VLerp` (`self.StartLocation`) (`self.EndLocation`) _newtrack_0) false false)))
    (else
      (`KismetSystemLibrary.PrintString` "you dont have got right key"))))

(fn `UserConstructionScript`
  (`PrimitiveComponent.SetMaterial` (`self.StaticMesh`) 0 (`self.Material`)))