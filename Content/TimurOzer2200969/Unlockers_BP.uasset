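; Unlocker pickup that removes the level's traps once the player touches the last one remaining.
; On box overlap by the third-person character, it adds the count of Unlockers_BP actors in the world to Number.
; If Number equals one, it destroys every swing axe, spike and smoke actor; otherwise it destroys itself.
; The construction script applies the Material variable to the cone mesh.
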(event `self.Box.OnComponentBeginOverlap`
  (params (OverlappedComponent :type "PrimitiveComponent Object Reference") (OtherActor :type "Actor Object Reference") (OtherComp :type "PrimitiveComponent Object Reference") (OtherBodyIndex :type Integer) (bFromSweep :type Boolean) (SweepResult :type "HitResult Structure (by ref)"))
  (bind _number (`self.Number`))
  (cast `/Game/TimurOzer2200969/BP_ThirdPersonCharacter` OtherActor)
  (bind _outactors (`GameplayStatics.GetAllActorsOfClass` "Unlockers_BP_C"))
  (for _ _outactors
    (`/Engine/EditorBlueprintResources/StandardMacros.IncrementInt` _number))
  (if (== _number 1)
    (bind _outactors_2 (`GameplayStatics.GetAllActorsOfClass` "/Game/TimurOzer2200969/SwingAxes_BP.SwingAxes_BP_C"))
    (for _array_element _outactors_2
      (`self.K2_DestroyActor` _array_element))
    (bind _outactors_3 (`GameplayStatics.GetAllActorsOfClass` "/Game/TimurOzer2200969/Spike_BP.Spike_BP_C"))
    (for _array_element_2 _outactors_3
      (`self.K2_DestroyActor` _array_element_2))
    (bind _outactors_4 (`GameplayStatics.GetAllActorsOfClass` "/Game/TimurOzer2200969/Smoke_BP.Smoke_BP_C"))
    (for _array_element_3 _outactors_4
      (`self.K2_DestroyActor` _array_element_3))
    (else
      (`self.K2_DestroyActor`))))

(fn `UserConstructionScript`
  (`PrimitiveComponent.SetMaterial` (`self.Cone`) 0 (`self.Material`)))