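; Smoke hazard actor that affects the third-person character while it is inside a Box trigger.
; On overlap it shows the character's PostProcess component and calls Hit through a DoOnce gate.
; Ending the overlap hides the PostProcess again and resets the gate, so the next entry can hit again.
; A random self-destroy branch exists but is unconnected and never runs.
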(event `self.ReceiveBeginPlay`)

(event `self.Box.OnComponentBeginOverlap`
  (params (OverlappedComponent :type "PrimitiveComponent Object Reference") (OtherActor :type "Actor Object Reference") (OtherComp :type "PrimitiveComponent Object Reference") (OtherBodyIndex :type Integer) (bFromSweep :type Boolean) (SweepResult :type "HitResult Structure (by ref)"))
  (bind _asbp_third_person_character (cast `/Game/TimurOzer2200969/BP_ThirdPersonCharacter` OtherActor))
  (`SceneComponent.SetVisibility` (`/Game/TimurOzer2200969/BP_ThirdPersonCharacter.PostProcess` _asbp_third_person_character) true false)
  (`/Engine/EditorBlueprintResources/StandardMacros.DoOnce` false :!label _label
    (:`Completed`
      (`/Game/TimurOzer2200969/BP_ThirdPersonCharacter.Hit` _asbp_third_person_character))))

(event `self.Box.OnComponentEndOverlap`
  (params (OverlappedComponent :type "PrimitiveComponent Object Reference") (OtherActor :type "Actor Object Reference") (OtherComp :type "PrimitiveComponent Object Reference") (OtherBodyIndex :type Integer))
  (bind _asbp_third_person_character (cast `/Game/TimurOzer2200969/BP_ThirdPersonCharacter` OtherActor))
  (`SceneComponent.SetVisibility` (`/Game/TimurOzer2200969/BP_ThirdPersonCharacter.PostProcess` _asbp_third_person_character) false false)
  (goto _label :!via `Reset`))

(fn `UserConstructionScript`)