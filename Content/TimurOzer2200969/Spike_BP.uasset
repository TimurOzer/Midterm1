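; Spike trap that randomly removes itself at BeginPlay, so only some placed spikes remain in a level.
; When the third-person character enters the Box, the mesh gains collision and a timeline moves it.
; When that timeline finishes, a stationary sphere trace around the actor calls Hit if it finds the character.
; Leaving the Box disables mesh collision and plays a second timeline in reverse to move the mesh.
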(event `self.ReceiveBeginPlay`
  (if (`KismetMathLibrary.RandomBool`)
    (`self.K2_DestroyActor`)))

(event `self.Box.OnComponentBeginOverlap`
  (params (OverlappedComponent :type "PrimitiveComponent Object Reference") (OtherActor :type "Actor Object Reference") (OtherComp :type "PrimitiveComponent Object Reference") (OtherBodyIndex :type Integer) (bFromSweep :type Boolean) (SweepResult :type "HitResult Structure (by ref)"))
  (bind _returnvalue (`self.K2_GetActorLocation`))
  (cast `/Game/TimurOzer2200969/BP_ThirdPersonCharacter` OtherActor)
  (`PrimitiveComponent.SetCollisionEnabled` (`self.StaticMesh`) "QueryAndPhysics")
  (bind (_direction _newtrack_0) (`Timeline|Timeline` :!via `PlayFromStart`)
    (:`Update`
      (`SceneComponent.K2_SetRelativeLocation` (`self.StaticMesh`) _newtrack_0 false false))
    (:`Finished`
      (bind _outhit (`KismetSystemLibrary.SphereTraceSingle` _returnvalue _returnvalue 300.0 "TraceTypeQuery1"))
      (bind _asbp_third_person_character (cast `/Game/TimurOzer2200969/BP_ThirdPersonCharacter` (`.HitActor` (`GameplayStatics.BreakHitResult` _outhit))))
      (`/Game/TimurOzer2200969/BP_ThirdPersonCharacter.Hit` _asbp_third_person_character))))

(event `self.Box.OnComponentEndOverlap`
  (params (OverlappedComponent :type "PrimitiveComponent Object Reference") (OtherActor :type "Actor Object Reference") (OtherComp :type "PrimitiveComponent Object Reference") (OtherBodyIndex :type Integer))
  (cast `/Game/TimurOzer2200969/BP_ThirdPersonCharacter` OtherActor)
  (`PrimitiveComponent.SetCollisionEnabled` (`self.StaticMesh`) "NoCollision")
  (bind (_direction _newtrack_0) (`Timeline|Timeline_0` :!via `ReverseFromEnd`)
    (:`Update`
      (`SceneComponent.K2_SetRelativeLocation` (`self.StaticMesh`) _newtrack_0 false false))))

(fn `UserConstructionScript`)